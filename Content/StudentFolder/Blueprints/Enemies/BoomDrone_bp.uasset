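; BoomDrone is an enemy drone that explodes on contact with the player or when shot.
; A ShipProjectile overlapping its hitbox destroys both, leaving only an explosion effect.
; A UnitController entering its radius trigger takes damage with explosion effect and sound, and the drone is destroyed after a short delay.
; UpdateChaseSpeed sets the floating pawn movement's max speed; no chase logic appears in these graphs.
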(event `self.Hitbox.OnComponentBeginOverlap`
  (params (OverlappedComponent :type "PrimitiveComponent Object Reference") (OtherActor :type "Actor Object Reference") (OtherComp :type "PrimitiveComponent Object Reference") (OtherBodyIndex :type Integer) (bFromSweep :type Boolean) (SweepResult :type "HitResult Structure (by ref)"))
  (bind _returnvalue (`ActorComponent.GetOwner` (`self.Sphere`)))
  (bind _asship_projectile_bp (cast `/Game/StudentFolder/Blueprints/Player/ShipProjectile_bp` OtherActor))
  (`self.K2_DestroyActor` _asship_projectile_bp)
  (`GameplayStatics.SpawnEmitterAtLocation` "/Game/StarterContent/Particles/P_Explosion.P_Explosion" (`self.K2_GetActorLocation` _returnvalue))
  (`self.K2_DestroyActor` _returnvalue))

(event `self.RadiusTrigger.OnComponentBeginOverlap`
  (params (OverlappedComponent :type "PrimitiveComponent Object Reference") (OtherActor :type "Actor Object Reference") (OtherComp :type "PrimitiveComponent Object Reference") (OtherBodyIndex :type Integer) (bFromSweep :type Boolean) (SweepResult :type "HitResult Structure (by ref)"))
  (bind _returnvalue (`ActorComponent.GetOwner` (`self.Sphere`)))
  (bind _returnvalue_2 (`self.K2_GetActorLocation` _returnvalue))
  ;[1 1 1] Explode when colliding with player
  (bind _asunit_controller_bp (cast `/Game/StudentFolder/Blueprints/Player/UnitController_bp` OtherActor))
  (`GameplayStatics.SpawnEmitterAtLocation` "/Game/StarterContent/Particles/P_Explosion.P_Explosion" _returnvalue_2)
  (`GameplayStatics.PlaySoundAtLocation` "/Game/StarterContent/Audio/Explosion01.Explosion01" _returnvalue_2 (struct) 1.0 1.0 0.0 null null null)
  (`GameplayStatics.ApplyDamage` _asunit_controller_bp 50.0 null self)
  (`KismetSystemLibrary.Delay` 0.5)
  (`self.K2_DestroyActor` _returnvalue))

(fn `UpdateChaseSpeed`
  (params (NewChaseSpeed :type "Float (double-precision)" :default 800.0))
  (set `FloatingPawnMovement.MaxSpeed` NewChaseSpeed (`self.FloatingPawnMovement`)))

(fn `UserConstructionScript`)