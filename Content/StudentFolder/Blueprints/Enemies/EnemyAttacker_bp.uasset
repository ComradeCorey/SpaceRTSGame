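; EnemyAttacker_bp is an enemy that turns toward and shoots at units it sees.
; When PawnSensing detects a UnitController_bp pawn, it interpolates its rotation toward that unit.
; It also spawns an EnemyProjectile_bp at ProjectileSpawnArea and launches it with an impulse along the cruiser mesh's forward vector.
; Two Delays toggle SpawnProjectile, so it fires on sightings for about a second, then pauses before firing again.
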(event `self.PawnSensing.OnSeePawn`
  (params (Pawn :type "Pawn Object Reference"))
  (bind _asunit_controller_bp (cast `/Game/StudentFolder/Blueprints/Player/UnitController_bp` Pawn))
  (`|ExecutionSequence`
    (:`then_0`
      (`self.K2_SetActorRotation` (`KismetMathLibrary.RInterpTo` (`self.K2_GetActorRotation`) (`KismetMathLibrary.FindLookAtRotation` (`self.K2_GetActorLocation`) (`self.K2_GetActorLocation` _asunit_controller_bp)) (`GameplayStatics.GetWorldDeltaSeconds`) 20.0)))
    (:`then_1`
      (if (`self.SpawnProjectile`)
        (bind _returnvalue (`|SpawnActorFromClass` "/Game/StudentFolder/Blueprints/Enemies/EnemyProjectile_bp.EnemyProjectile_bp_C" (`SceneComponent.K2_GetComponentToWorld` (`self.ProjectileSpawnArea`)) "Undefined" "OverrideRootScale" null 10.0 null))
        (`PrimitiveComponent.AddImpulse` (`/Game/StudentFolder/Blueprints/Enemies/EnemyProjectile_bp.Bullet` _returnvalue) (* (`SceneComponent.GetForwardVector` (`self.StaticMesh_synth_cruiser`)) (`self.ShotForce`)) "None" true)
        (`KismetSystemLibrary.Delay` 1.0)
        (set `self.SpawnProjectile` false)
        (`KismetSystemLibrary.Delay` 2.5)
        (set `self.SpawnProjectile` true)))))

(fn `UserConstructionScript`)