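; Enemy Warper actor that turns toward a seen player unit and shoots it, and is destroyed when its clamped health runs out.
; Pawn sensing drives the rotation and spawns impulse-launched projectiles, with chained delays toggling firing off and back on.
; BeginPlay caches three move points and picks one at random.
; A timeline meant to lerp between them with particle toggling is never started, so the warp movement does not run.
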(event `self.ReceiveAnyDamage`
  (params (Damage :type "Float (single-precision)") (DamageType :type "DamageType Object Reference") (InstigatedBy :type "Controller Object Reference") (DamageCauser :type "Actor Object Reference"))
  (bind _output_get (set `self.WarperHealth` (`KismetMathLibrary.FClamp` (- (`self.WarperHealth`) Damage) 0.0 75.0)))
  (`KismetSystemLibrary.PrintString` (`KismetStringLibrary.Concat_StrStr` "Warper HP: " (`KismetStringLibrary.Conv_DoubleToString` _output_get)) true true (struct :`R` 0.228102 :`G` 1.0 :`A` 1.0))
  (if (<= _output_get 0.0)
    (`self.K2_DestroyActor`)))

(event `self.PawnSensing.OnSeePawn`
  (params (Pawn :type "Pawn Object Reference"))
  ;[1 1 1] Look and Shoot
  (bind _asunit_controller_bp (cast `/Game/StudentFolder/Blueprints/Player/UnitController_bp` Pawn))
  (`|ExecutionSequence`
    (:`then_0`
      (`self.K2_SetActorRelativeRotation` (`KismetMathLibrary.RInterpTo` (`self.K2_GetActorRotation`) (`KismetMathLibrary.FindLookAtRotation` (`self.K2_GetActorLocation`) (`self.K2_GetActorLocation` _asunit_controller_bp)) (`GameplayStatics.GetWorldDeltaSeconds`) 20.0)))
    (:`then_1`
      (if (`self.SpawnProjectile`)
        (bind _returnvalue (`|SpawnActorFromClass` "/Game/StudentFolder/Blueprints/Enemies/EnemyProjectile_bp.EnemyProjectile_bp_C" (`SceneComponent.K2_GetComponentToWorld` (`self.ProjectileSpawnArea`)) "Undefined" "OverrideRootScale" null 10.0 null))
        (`PrimitiveComponent.AddImpulse` (`/Game/StudentFolder/Blueprints/Enemies/EnemyProjectile_bp.Bullet` _returnvalue) (* (`SceneComponent.GetForwardVector` (`self.StaticMesh_synth_cruiser`)) (`self.ShotForce`)) "None" true)
        (`KismetSystemLibrary.Delay` 1.0)
        (set `self.SpawnProjectile` false)
        (`KismetSystemLibrary.Delay` 2.5)
        (set `self.SpawnProjectile` true)))))

(event `self.ReceiveBeginPlay`
  ;[1 1 1] Set Patrol Points
  (set `self.MovePoints` (`|MakeArray` (`SceneComponent.K2_GetComponentLocation` (`self.MovePoint1`)) (`SceneComponent.K2_GetComponentLocation` (`self.MovePoint2`)) (`SceneComponent.K2_GetComponentLocation` (`self.MovePoint3`))))
  (`self.GetRandomLocation`))

(fn `GetRandomLocation`
  (set `self.CurrentMovePoint` (`KismetMathLibrary.RandomInteger` (`KismetArrayLibrary.Array_Length` (`self.MovePoints`)))))

(fn `UserConstructionScript`)