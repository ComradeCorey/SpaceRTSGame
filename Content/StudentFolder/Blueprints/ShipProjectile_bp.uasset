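; ShipProjectile_bp is a player projectile that damages enemies and expires after a short lifetime.
; On overlap with an EnemyController_bp actor, it applies DamageDealt and destroys itself.
; Every Tick, it casts the player pawn to UnitController_bp and sets the Bullet component to ignore it when moving.
; Activation of ProjectileMovement starts a one-second looping timer whose BulletDecay event destroys the projectile.
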(event `self.ReceiveActorBeginOverlap`
  (params (OtherActor :type "Actor Object Reference"))
  ;[1 1 1] Deal Damage to Enemy
  (bind _asenemy_controller_bp (cast `/Game/StudentFolder/Blueprints/EnemyController_bp` OtherActor))
  (`GameplayStatics.ApplyDamage` _asenemy_controller_bp (`self.DamageDealt`) null self)
  (`self.K2_DestroyActor`))

(event `self.ReceiveTick`
  (params (DeltaSeconds :type "Float (single-precision)"))
  (bind _asunit_controller_bp (cast `/Game/StudentFolder/Blueprints/UnitController_bp` (`GameplayStatics.GetPlayerPawn` 0)))
  (`PrimitiveComponent.IgnoreActorWhenMoving` (`self.Bullet`) _asunit_controller_bp true))

(event `self.ProjectileMovement.OnComponentActivated`
  (params (Component :type "ActorComponent Object Reference") (bReset :type Boolean))
  (`KismetSystemLibrary.K2_SetTimerDelegate` (delegate `BulletDecay`) 1.0 true))

(event `BulletDecay`
  (`self.K2_DestroyActor`))

(fn `UserConstructionScript`)