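; Player ship controller Blueprint with click-to-move navigation and automatic firing at an enemy.
; Left click calls SimpleMoveToLocation on the point under the cursor, which BeginPlay makes visible.
; Tick updates a range check against a single Enemy reference and smoothly turns the Player component toward it while in range.
; A self-calling retriggerable-delay loop spawns ShipProjectile_bp at the FirePoint socket when in range, otherwise polls again.
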(event `Key|LeftMouseButton`
  (params (Key :type "Key Structure"))
  (bind _returnvalue (`GameplayStatics.GetPlayerController` 0))
  ;[1 1 1] Move Ship to Mouse Location
  (:`Pressed`
    (`AIBlueprintHelperLibrary.SimpleMoveToLocation` _returnvalue (`.Location` (`GameplayStatics.BreakHitResult` (`PlayerController.GetHitResultUnderCursorByChannel` _returnvalue "TraceTypeQuery2" true))))))

(event `self.ReceiveBeginPlay`
  (`|ExecutionSequence`
    (:`then_0`
      ;[1 1 1] Move Ship to Mouse Location
      (set `PlayerController.bShowMouseCursor` true (`GameplayStatics.GetPlayerController` 0)))
    (:`then_1`
      (`self.ShootEnemy`))))

(event `self.ReceiveTick`
  (params (DeltaSeconds :type "Float (single-precision)"))
  (set `self.DeltaTime` DeltaSeconds)
  (`self.GunRotation`)
  (`self.EnemyRange`))

(event `GunRotation`
  (bind _player (`self.Player`))
  ;[1 1 1] Rotate Ships to Face Enemies
  (if (`self.InRange`)
    (`SceneComponent.K2_SetWorldRotation` _player (`KismetMathLibrary.RInterpTo` (`SceneComponent.K2_GetComponentRotation` _player) (`KismetMathLibrary.MakeRotator` 0.0 (.pitch (`KismetMathLibrary.FindLookAtRotation` (`SceneComponent.K2_GetComponentLocation` (`self.Player`)) (`self.K2_GetActorLocation` (`self.Enemy`)))) (.yaw (`KismetMathLibrary.FindLookAtRotation` (`SceneComponent.K2_GetComponentLocation` (`self.Player`)) (`self.K2_GetActorLocation` (`self.Enemy`))))) (`self.DeltaTime`) (`self.RotationSpeed`)) false false)))

(event `EnemyRange`
  ;[1 1 1] Check if Enemies are in Range
  (if (< (`self.GetDistanceTo` self (`self.Enemy`)) (`self.AttackRange`))
    (set `self.InRange` true)
    (else
      (set `self.InRange` false))))

(event `ShootEnemy`
  ;[1 1 1] Shoot Enemies
  (if (`self.InRange`)
    (`|SpawnActorFromClass` "/Game/StudentFolder/Blueprints/ShipProjectile_bp.ShipProjectile_bp_C" (`SceneComponent.GetSocketTransform` (`self.Player`) "FirePoint" "RTS_World") "Undefined" "OverrideRootScale" null 10.0 null)
    (`KismetSystemLibrary.RetriggerableDelay` (`self.FireRate`))
    (`self.ShootEnemy`)
    (else
      (`KismetSystemLibrary.RetriggerableDelay` 0.5)
      (`self.ShootEnemy`))))

(fn `UserConstructionScript`)