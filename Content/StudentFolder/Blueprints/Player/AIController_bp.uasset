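; AI controller Blueprint that drives a ship pawn through two commands: attack an area and move to a location.
; The attack event waits briefly, prints a debug message, then spawns a scaled-down ship projectile offset along world X from the pawn, rotated toward the target.
; The move event waits briefly, then paths the ship to the goal with SimpleMoveToLocation.
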(event `/Game/StudentFolder/Blueprints/InterfaceRTS_bp.ShipAttackAt`
  (params (Area :type "Vector Structure"))
  (bind _returnvalue (`self.K2_GetActorLocation` (`self.K2_GetPawn`)))
  (`KismetSystemLibrary.Delay` 0.5)
  (`KismetSystemLibrary.PrintString` "Firing" true true (struct :`R` 0.754833 :`B` 1.0 :`A` 1.0) 1.0)
  (`|SpawnActorFromClass` "/Game/StudentFolder/Blueprints/Player/ShipProjectile_bp.ShipProjectile_bp_C" (`KismetMathLibrary.MakeTransform` (+ _returnvalue (100.0 0.0 0.0)) (`KismetMathLibrary.FindLookAtRotation` _returnvalue Area) (0.5 0.5 0.5)) "Undefined" "OverrideRootScale" null 10.0 null))

(event `/Game/StudentFolder/Blueprints/InterfaceRTS_bp.MoveShipTo`
  (params (Location :type "Vector Structure"))
  ;[1 1 1] Move ship to location
  (`KismetSystemLibrary.Delay` 0.25)
  (`AIBlueprintHelperLibrary.SimpleMoveToLocation` self Location))

(fn `UserConstructionScript`)