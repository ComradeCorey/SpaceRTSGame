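; Player camera for a click-to-command ship game, handling unit selection, orders and view control.
; Left-clicking a Pawn under the cursor selects it, opens Gates for orders and glides the Rotpoint pivot to it.
; Right-click sends a navmesh-projected move with heading while the pivot follows over distance-scaled time; Fire Toggle sends an attack at the cursor.
; Middle-mouse drag rotates the pivot with roll zeroed; the wheel zooms the camera within limits.
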(event `InputAction|Fire Toggle`
  (params (Key :type "Key Structure"))
  (:`Pressed`
    (`/Engine/EditorBlueprintResources/StandardMacros.Gate` true :!label _label
      (:`Exit`
        (message `/Game/StudentFolder/Blueprints/InterfaceRTS_bp.ShipAttackAt` (stale `Key|LeftMouseButton` _aspawn) (`.Location` (`GameplayStatics.BreakHitResult` (`PlayerController.GetHitResultUnderCursorByChannel` (`GameplayStatics.GetPlayerController` 0) "TraceTypeQuery1" false))))))))

(event `Key|LeftMouseButton`
  (params (Key :type "Key Structure"))
  (:`Pressed`
    (bind _aspawn (cast `Pawn` (`.HitActor` (`GameplayStatics.BreakHitResult` (`PlayerController.GetHitResultUnderCursorByChannel` (`GameplayStatics.GetPlayerController` 0) "TraceTypeQuery1" false))))
      (:`then`
        (goto _label :!via `Open`))
      (:`CastFailed`
        (goto _label :!via `Close`)))))

(event `Key|LeftMouseButton`
  (params (Key :type "Key Structure"))
  (bind (_bblockinghit _binitialoverlap _time _distance _location _impactpoint _normal _impactnormal _physmat _hitactor) (`GameplayStatics.BreakHitResult` (`PlayerController.GetHitResultUnderCursorByChannel` (`GameplayStatics.GetPlayerController` 0) "TraceTypeQuery1" false)))
  (bind _projectedlocation (`NavigationSystemV1.K2_ProjectPointToNavigation` _location))
  (bind _returnvalue (- _projectedlocation (`self.unitpos`)))
  ;[1 1 1] Selecting a Unit to Move
  (:`Pressed`
    (`|ExecutionSequence`
      (:`then_0`
        (bind _aspawn (cast `Pawn` _hitactor)
          (:`then`
            (set `self.selected ship` _aspawn)
            (set `self.first_ship_selected` true)
            (`KismetSystemLibrary.PrintString` "Unit Selected")
            (goto _label_2 :!via `Open`))
          (:`CastFailed`
            (goto _label_2 :!via `Close`))))
      (:`then_1`
        ;[1 1 1] cam mvrt
        (cast `Pawn` _hitactor)
        (`KismetSystemLibrary.MoveComponentTo` (`self.rotpoint`) (`self.K2_GetActorLocation` _hitactor) (`self.camrotation`) true true 1.0)))))

(event `Key|RightMouseButton`
  (params (Key :type "Key Structure"))
  (bind _projectedlocation (`NavigationSystemV1.K2_ProjectPointToNavigation` (`.Location` (`GameplayStatics.BreakHitResult` (`PlayerController.GetHitResultUnderCursorByChannel` (`GameplayStatics.GetPlayerController` 0) "TraceTypeQuery1" false)))))
  (bind _returnvalue (- _projectedlocation (`self.unitpos`)))
  ;[1 1 1] Selecting a Unit to Move
  (:`Pressed`
    (if (`self.first_ship_selected`)
      (set `self.unitpos` (`self.K2_GetActorLocation` (`self.selected ship`))))
    (`/Engine/EditorBlueprintResources/StandardMacros.Gate` true :!label _label_2
      (:`Exit`
        (message `/Game/StudentFolder/Blueprints/InterfaceRTS_bp.MoveShipTo` (stale `Key|LeftMouseButton` _aspawn) _projectedlocation (`self.unitpos`) (`KismetMathLibrary.MakeRotator` 0.0 0.0 (`KismetMathLibrary.RadiansToDegrees` (`KismetMathLibrary.Vector_HeadingAngle` _returnvalue))))
        (`KismetSystemLibrary.MoveComponentTo` (`self.rotpoint`) _projectedlocation (`self.camrotation`) true true (* (`KismetMathLibrary.Sqrt` (+ (`KismetMathLibrary.Square` (.x _returnvalue)) (`KismetMathLibrary.Square` (.y _returnvalue)))) 0.0045))))))

(event `InputAxisKey|MouseY`
  (params (AxisValue :type "Float (single-precision)"))
  (bind _rotpoint (`self.rotpoint`))
  (bind _returnvalue (`KismetMathLibrary.MakeRotator` 0.0 (.pitch (`SceneComponent.K2_GetComponentRotation` _rotpoint)) (.yaw (`SceneComponent.K2_GetComponentRotation` _rotpoint))))
  ;[1 1 1] camera rotation
  (if (`self.MiddleMouse`) :!label _label_3
    (`SceneComponent.K2_AddLocalRotation` _rotpoint (`KismetMathLibrary.MakeRotator` 0.0 (* AxisValue 2.0) (* (stale `InputAxisKey|MouseX` AxisValue) 2.0)) false false)
    (`SceneComponent.K2_SetWorldRotation` _rotpoint _returnvalue false false)
    (set `self.camrotation` _returnvalue)))

(event `Key|MouseScrollUp`
  (params (Key :type "Key Structure"))
  (bind _camera (`self.Camera`))
  ;[1 1 1] scroll in and out
  (:`Pressed`
    (if (not (>= (.x (`self.limit`)) -250.0))
      (`SceneComponent.K2_AddLocalOffset` _camera (50.0 0.0 0.0) false false)
      (set `self.limit` (`SceneComponent.RelativeLocation` _camera)))))

(event `InputAxisKey|MouseX`
  (params (AxisValue :type "Float (single-precision)"))
  ;[1 1 1] camera rotation
  (goto _label_3))

(event `Key|MouseScrollDown`
  (params (Key :type "Key Structure"))
  (bind _camera (`self.Camera`))
  ;[1 1 1] scroll in and out
  (:`Pressed`
    (if (not (<= (.x (`self.limit`)) -3200.0))
      (`SceneComponent.K2_AddLocalOffset` _camera (-50.0 0.0 0.0) false false)
      (set `self.limit` (`SceneComponent.RelativeLocation` _camera)))))

(event `Key|MiddleMouseButton`
  (params (Key :type "Key Structure"))
  ;[1 1 1] camera rotation
  ;;[1 1 1] Middle Mouse to enable camera movement
  (:`Pressed`
    (set `self.MiddleMouse` true))
  (:`Released`
    (set `self.MiddleMouse` false)))

(fn `UserConstructionScript`)