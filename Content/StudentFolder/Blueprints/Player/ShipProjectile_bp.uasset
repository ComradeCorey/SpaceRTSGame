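; ShipProjectile_bp is a projectile that damages whatever it hits, then destroys itself.
; Damage is a base value plus a rounded random crit bonus, printed to screen as debug output.
; A timer started on ProjectileMovement activation destroys the projectile after one second.
; Every tick, if the owner is a BoomDrone_bp, it sets that drone's RadiusTrigger to ignore itself when moving.
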(event `self.ReceiveHit`
  (params (MyComp :type "PrimitiveComponent Object Reference") (Other :type "Actor Object Reference") (OtherComp :type "PrimitiveComponent Object Reference") (bSelfMoved :type Boolean) (HitLocation :type "Vector Structure") (HitNormal :type "Vector Structure") (NormalImpulse :type "Vector Structure") (Hit :type "HitResult Structure (by ref)"))
  ;[1 1 1] Send Damage on Hit
  (bind _output_get (set `self.DamageToDeal` (+ (`self.DamageDealt`) (`KismetMathLibrary.Conv_IntToDouble` (`KismetMathLibrary.Round` (`KismetMathLibrary.RandomFloatInRange` 1.0 (`self.AdditionalDamageCrit`)))))))
  (bind _returnvalue (`GameplayStatics.ApplyDamage` Other _output_get))
  (`KismetSystemLibrary.PrintString` (`KismetStringLibrary.Conv_DoubleToString` _output_get) true true (struct :`G` 0.66 :`B` 1.0 :`A` 1.0) _returnvalue)
  (`self.K2_DestroyActor`))

(event `self.ProjectileMovement.OnComponentActivated`
  (params (Component :type "ActorComponent Object Reference") (bReset :type Boolean))
  (`KismetSystemLibrary.K2_SetTimerDelegate` (delegate `BulletDecay`) 1.0 true))

(event `BulletDecay`
  (`self.K2_DestroyActor`))

(event `self.ReceiveTick`
  (params (DeltaSeconds :type "Float (single-precision)"))
  (bind _asboom_drone_bp (cast `/Game/StudentFolder/Blueprints/Enemies/BoomDrone_bp` (`self.GetOwner`)))
  (bind _radiustrigger (`/Game/StudentFolder/Blueprints/Enemies/BoomDrone_bp.RadiusTrigger` _asboom_drone_bp))
  (`PrimitiveComponent.IgnoreComponentWhenMoving` _radiustrigger _radiustrigger true))

(fn `UserConstructionScript`)