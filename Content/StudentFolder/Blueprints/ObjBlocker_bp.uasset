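; ObjBlocker_bp is an anomaly blocker that breaks down as its linked objective objects are captured to an area.
; On BeginPlay it binds both objectives' captured events to TakeDamage, which subtracts orb damage from AnomalyHealth.
; At zero health, a delayed sequence adjusts particle time dilation, pulls the rock into the anomaly, activates a particle effect and destroys the actor.
; An OrbStages event for slowing the bloom at partial health is never called.
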(event `self.ReceiveBeginPlay`
  (add `/Game/StudentFolder/Blueprints/CapturePoint_bp.CapturedToArea` (`self.ObjectiveObject1`) (delegate `TakeDamage`))
  (add `/Game/StudentFolder/Blueprints/CapturePoint_bp.CapturedToArea` (`self.ObjectiveObject2`) (delegate `TakeDamage`)))

(event `TakeDamage`
  (params (DamageToOrb :type "Float (double-precision)"))
  (bind _anomalyhealth (`self.AnomalyHealth`))
  (set `self.AnomalyHealth` (- _anomalyhealth DamageToOrb))
  (if (<= _anomalyhealth 0.0)
    (bind _output_get (set `self.isDead` true))
    (if _output_get
      (`KismetSystemLibrary.Delay` 1.0)
      (set `ParticleSystemComponent.CustomTimeDilation` 1.0 (`self.ParticleBloom`))
      (`KismetSystemLibrary.Delay` 2.0)
      (`ActorComponent.K2_DestroyComponent` (`self.RockParticle`))
      (`KismetSystemLibrary.MoveComponentTo` (`self.Rock`) (`SceneComponent.RelativeLocation` (`self.Anomaly`)) (struct) true true 1.0)
      (`ActorComponent.K2_DestroyComponent` (`self.Rock`))
      (`ActorComponent.SetActive` (`self.ParticleSystem`) true false)
      (`KismetSystemLibrary.Delay` 0.5)
      (`self.K2_DestroyActor`))))

(event `OrbStages`
  (params (OrbDamaged :type Boolean))
  (if (== (`self.AnomalyHealth`) 50.0)
    (set `ParticleSystemComponent.CustomTimeDilation` 0.75 (`self.ParticleBloom`))))

(fn `UserConstructionScript`)